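; Game instance for the Endless game that holds the save data and restores the enemy kill count.
; On Init it loads the save slot into SaveGameData, or creates a fresh save object in memory when none exists.
; LoadGameModeData copies the saved kill count into the game mode passed to it and prints the value.
; The file only reads saves and never writes one to disk.
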(event EventInit
  (bind _returnvalue (SaveGame|DoesSaveGameExist (Variables|Default|GetSaveSlotName)))
  (if _returnvalue
    (bind _returnvalue_2 (SaveGame|LoadGamefromSlot (Variables|Default|GetSaveSlotName)))
    (bind _asbp_save_game_object (Utilities|Casting|CastToBP_SaveGameObject _returnvalue_2))
    (Variables|Default|SetSaveGameData _asbp_save_game_object)
    (else
      (bind _returnvalue_3 (SaveGame|CreateSaveGameObject "/Game/BP_SaveGameObject.BP_SaveGameObject_C"))
      (Variables|Default|SetSaveGameData _returnvalue_3)
      (Development|PrintString "No Save"))))

(fn LoadGameModeData
  (params (GameMode :type BP%20Endless%20Game%20Mode%20Object%20Reference))
  (bind _output_get (Variables|/Script/SImpleShooter.EndlessGameMode|SetNumberOfEnemiesKilled GameMode (Variables|/Game/BP_SaveGameObject.BP_SaveGameObject_C|GetEnemiesKilled (Variables|Default|GetSaveGameData))))
  (Development|PrintString (Utilities|String|ToString(Integer) _output_get)))